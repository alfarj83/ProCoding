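; BP_Controller is a controller Blueprint that sets up player input and passes mouse-driven rotation to the player character.
; On BeginPlay it adds the Inputmapping context to the Enhanced Input local player subsystem.
; Every Tick it reads ReturnMouseData from MouseControl and writes it to the BP_Character's Rotator variable.
; Leftover mouse-axis, pitch-clamp and debug-print nodes are disconnected and never run.
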(event `self.ReceiveBeginPlay`
  (`EnhancedInputSubsystemInterface.AddMappingContext` (subsystem `EnhancedInputLocalPlayerSubsystem`) "/Game/Inputs/Inputmapping.Inputmapping" 0 (struct)))

(event `self.ReceiveTick`
  (params (DeltaSeconds :type "Float (single-precision)"))
  (bind _returnvalue (`MouseControlComponent.ReturnMouseData` (`self.MouseControl`)))
  (bind _asbp_character (cast `/Game/StarterContent/Blueprints/BP_Character` (`GameplayStatics.GetPlayerCharacter` 0)))
  (set `/Game/StarterContent/Blueprints/BP_Character.Rotator` _returnvalue _asbp_character))

(fn `UserConstructionScript`)