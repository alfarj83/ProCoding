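; Parent Blueprint for world props that the player picks up into the character's inventory.
; On BeginPlay it hands its Sphere to the PropCollisionInput component, then polls every Tick for player proximity and the pickup action.
; On pickup it spawns an ObjectType actor far outside the playable space, owned by the character, adds it to Inventory and destroys the prop.
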(event `self.ReceiveBeginPlay`
  (`PropCollisionInputComponent.SetCollisionReference` (`self.PropCollisionInput`) (`self.Sphere`)))

(event `self.ReceiveTick`
  (params (DeltaSeconds :type "Float (single-precision)"))
  (bind _returnvalue (`PropCollisionInputComponent.IsPlayerNear` (`self.PropCollisionInput`)))
  (if (and _returnvalue (`|GetInputActionValue`))
    (bind _returnvalue_2 (`PropCollisionInputComponent.ReturnCharacterReference` (`self.PropCollisionInput`)))
    (bind _asbp_character (cast `/Game/Rimanaru/Blueprints/BP_Character` _returnvalue_2))
    (bind _returnvalue_3 (`|SpawnActorFromClass` (`self.ObjectType`) (`KismetMathLibrary.MakeTransform` (-1000000.0 -1000000.0 -1000000.0)) "Undefined" "MultiplyWithRoot" _asbp_character null))
    (`InventoryComponent.AddItem` (`/Game/Rimanaru/Blueprints/BP_Character.Inventory` _asbp_character) _returnvalue_3)
    (`self.K2_DestroyActor`)))

(fn `UserConstructionScript`)