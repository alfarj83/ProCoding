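; Flashlight pickup prop that lets a nearby character add a flashlight to their inventory.
; On BeginPlay it hands its Sphere to PropCollisionInput for proximity detection and spawns a BP_FlashlightItem at world origin as the item it grants.
; Tick polls for a near player and the pickup action, then passes that item to the BP_Character's inventory, without destroying or hiding the prop.
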(event `self.ReceiveBeginPlay`
  (`PropCollisionInputComponent.SetCollisionReference` (`self.PropCollisionInput`) (`self.Sphere`))
  (bind _returnvalue (`|SpawnActorFromClass` "/Game/Rimanaru/Blueprints/Items/BP_FlashlightItem.BP_FlashlightItem_C" (`KismetMathLibrary.MakeTransform` (0.0 0.0 0.0)) "Undefined" "MultiplyWithRoot" null null))
  (set `self.ItemReference` _returnvalue))

(event `self.ReceiveTick`
  (params (DeltaSeconds :type "Float (single-precision)"))
  (bind _returnvalue (`PropCollisionInputComponent.IsPlayerNear` (`self.PropCollisionInput`)))
  (if (and _returnvalue (`|GetInputActionValue`))
    (bind _asbp_character (cast `/Game/Rimanaru/Blueprints/BP_Character` (`PropCollisionInputComponent.CharacterNear` (`self.PropCollisionInput`))))
    (`InventoryComponent.AddItem` (`/Game/Rimanaru/Blueprints/BP_Character.InventoryReference` _asbp_character) (`self.ItemReference`))))

(fn `UserConstructionScript`)