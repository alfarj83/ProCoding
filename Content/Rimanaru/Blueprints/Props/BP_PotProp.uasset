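; BP_PotProp is an interactable pot prop that gives the player a flashlight item.
; On BeginPlay it registers its sphere with a PotCollisionComponent, which tracks nearby characters.
; Tick polls that component and the pickup action, then spawns a BP_FlashlightItem at the world origin and adds it to the nearby BP_Character's inventory.
; The pot has no one-time guard and stays in place after pickup.
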(event `self.ReceiveBeginPlay`
  (`PropCollisionInputComponent.SetCollisionReference` (`self.PotCollisionComponent`) (`self.PotSphere`)))

(event `self.ReceiveTick`
  (params (DeltaSeconds :type "Float (single-precision)"))
  (bind _returnvalue (`PropCollisionInputComponent.IsPlayerNear` (`self.PotCollisionComponent`)))
  (if (and _returnvalue (`|GetInputActionValue`))
    (bind _asbp_character (cast `/Game/Rimanaru/Blueprints/BP_Character` (`PropCollisionInputComponent.CharacterNear` (`self.PotCollisionComponent`))))
    (bind _returnvalue_2 (`|SpawnActorFromClass` "/Game/Rimanaru/Blueprints/Items/BP_FlashlightItem.BP_FlashlightItem_C" (`KismetMathLibrary.MakeTransform` (0.0 0.0 0.0)) "Undefined" "MultiplyWithRoot" null null))
    (`InventoryComponent.AddItem` (`/Game/Rimanaru/Blueprints/BP_Character.Inventory` _asbp_character) _returnvalue_2)))

(fn `UserConstructionScript`)