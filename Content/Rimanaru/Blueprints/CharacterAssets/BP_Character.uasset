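; Player character Blueprint that handles Enhanced Input look and movement, inventory slot swapping and backpack creation.
; BeginPlay binds to the player state's inventory-change event and spawns a BP_Backpack, assigning it to the Inventory.
; Swap input stores the slot and sets StartSwapAnim, while SwapItemFunction separately applies the zero-based index change.
; Completing the inventory action clears the player state's inventory state; InventoryStateAction is only a debug print.
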(event `EnhancedInput|/Game/Rimanaru/Inputs/IA_MouseInput`
  (params (ActionValue :type "Vector2D Structure") (ElapsedSeconds :type "Float (double-precision)") (TriggeredSeconds :type "Float (double-precision)") (InputAction :type "InputAction Object Reference" :default "/Game/Rimanaru/Inputs/IA_MouseInput.IA_MouseInput"))
  ;[1 1 1] Setting Controls Up
  (:`Triggered`
    (`self.AddControllerPitchInput` (* ActionValue_Y -0.5))
    (`self.AddControllerYawInput` (* ActionValue_X 0.5))))

(event `EnhancedInput|/Game/Rimanaru/Inputs/IA_MoveButtons`
  (params (ActionValue :type "Vector2D Structure") (ElapsedSeconds :type "Float (double-precision)") (TriggeredSeconds :type "Float (double-precision)") (InputAction :type "InputAction Object Reference" :default "/Game/Rimanaru/Inputs/IA_MoveButtons.IA_MoveButtons"))
  (bind (_returnvalue_roll _returnvalue_pitch _returnvalue_yaw) (`KismetMathLibrary.BreakRotator` (`self.GetControlRotation`)))
  (bind (_x _y) (`KismetMathLibrary.BreakVector2D` ActionValue))
  (bind (_returnvalue_roll_2 _returnvalue_pitch_2 _returnvalue_yaw_2) (`KismetMathLibrary.BreakRotator` (`self.GetControlRotation`)))
  ;[1 1 1] Setting Controls Up
  (:`Triggered`
    (`self.AddMovementInput` (`KismetMathLibrary.GetRightVector` (`KismetMathLibrary.MakeRotator` _returnvalue_roll 0.0 _returnvalue_yaw)) _x)
    (`self.AddMovementInput` (`KismetMathLibrary.GetForwardVector` (`KismetMathLibrary.MakeRotator` 0.0 0.0 _returnvalue_yaw_2)) _y)))

(event `EnhancedInput|/Game/Rimanaru/Inputs/IA_InventorySwapping`
  (params (ActionValue :type "Float (double-precision)") (ElapsedSeconds :type "Float (double-precision)") (TriggeredSeconds :type "Float (double-precision)") (InputAction :type "InputAction Object Reference" :default "/Game/Rimanaru/Inputs/IA_InventorySwapping.IA_InventorySwapping"))
  (:`Started`
    (`self.Inventory Reference`
      (:`then`
        (if (not (`self.StartSwapAnim`))
          (set `self.ItemToSwapTo` (`KismetMathLibrary.FTrunc` ActionValue))
          (set `self.StartSwapAnim` true)))
      (:`else`))))

(event `self.ReceiveBeginPlay`
  (bind _asparent_player_state_class (cast `ParentPlayerStateClass` (`self.PlayerState`)))
  (bind _output_get (set `self.PlayerStateReference` _asparent_player_state_class))
  (add `ParentPlayerStateClass.OnInventoryStateChange` _output_get (`|CreateDelegate` :!event `InventoryStateAction`))
  (`self.CreateBackpack`))

(event `EnhancedInput|/Game/Rimanaru/Inputs/IA_InventoryAction`
  (params (ActionValue :type Boolean) (ElapsedSeconds :type "Float (double-precision)") (TriggeredSeconds :type "Float (double-precision)") (InputAction :type "InputAction Object Reference" :default "/Game/Rimanaru/Inputs/IA_InventoryAction.IA_InventoryAction"))
  (:`Completed`
    (`ParentPlayerStateClass.SetInventoryState` (`self.PlayerStateReference`) false)))

(fn `CreateBackpack`
  (set `self.Inventory Reference` (`self.Inventory`))
  (bind _returnvalue (`|SpawnActorFromClass` "/Game/Rimanaru/Blueprints/CharacterAssets/BP_Backpack.BP_Backpack_C" (`KismetMathLibrary.MakeTransform` (0.0 0.0 0.0)) "Undefined" "MultiplyWithRoot" null self null))
  (bind _inventory_reference (`self.Inventory Reference`)
    (:`then`
      (set `Inventory.Backpack` _returnvalue _inventory_reference))
    (:`else`)))

(fn `InventoryStateAction`
  (params (IsInInventory :type Boolean))
  (`KismetSystemLibrary.PrintString` "Hello"))

(fn `RetrievePlayerIndex`
  (returns (PlayerIndex :type Integer))
  (bind _asbp_controller (cast `/Game/Rimanaru/Blueprints/BP_Controller` (`self.GetController`))
    (:`then`
      (bind _playerindex (`TurnBasedBlueprintLibrary.GetMyPlayerIndex` _asbp_controller))
      (return _playerindex))
    (:`CastFailed`
      (`KismetSystemLibrary.PrintString` "Can't Find Player Index"))))

(fn `SwapItemFunction`
  (locals (ItemReference :type "ItemParentClass Object Reference"))
  (bind _inventory_reference (`self.Inventory Reference`)
    (:`then`
      (`Inventory.ChangeInventoryItem` _inventory_reference (- (`self.ItemToSwapTo`) 1)))
    (:`else`)))

(fn `UserConstructionScript`)