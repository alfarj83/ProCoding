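; Player camera manager that adds head bobbing while BP_Character walks.
; The character's walk start and end events drive a timeline, whose value becomes a rotation offset.
; On finish, the timeline flips direction to ping-pong while walking, and stops at zero once movement ends.
; BlueprintUpdateCamera follows the character's camera component, adding location and rotation offsets with a fixed FOV.
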(event `StartHeadBobbing`
  (if (`self.isPlayerMoving`)
    (if (`self.Direction`)
      (bind (_direction _bobbinginterpolationvalue) (`Timeline|Timeline` :!label _label)
        (:`Update`
          (set `self.Bobbing Interpolation Value` _bobbinginterpolationvalue)
          (set `self.RotationAdditive` (`KismetMathLibrary.MakeRotator` 0.0 (* (`self.Bobbing Interpolation Value`) 1.0))))
        (:`Finished`
          (`self.FResetTimeline` _bobbinginterpolationvalue)))
      (else
        (goto _label :!via `Reverse`)))
    (else
      (goto _label :!via `Reverse`))))

(event `ForceStop`
  (goto _label :!via `Stop`))

(event `self.ReceiveBeginPlay`
  (bind _asbp_character (cast `/Game/Rimanaru/Blueprints/CharacterAssets/BP_Character` (`GameplayStatics.GetPlayerCharacter` 0)))
  (add `/Game/Rimanaru/Blueprints/CharacterAssets/BP_Character.OnStartWalking` _asbp_character (delegate `WalkingCamDataStart`))
  (add `/Game/Rimanaru/Blueprints/CharacterAssets/BP_Character.OnEndWalking` _asbp_character (delegate `WalkingCamDataEnd`)))

(event `WalkingCamDataStart`
  (set `self.isPlayerMoving` true)
  (`self.StartHeadBobbing`))

(event `WalkingCamDataEnd`
  (set `self.isPlayerMoving` false)
  (`self.StartHeadBobbing`))

(fn `BlueprintUpdateCamera`
  (params (CameraTarget :type "Actor Object Reference"))
  (returns (NewCameraLocation :type "Vector Structure") (NewCameraRotation :type "Rotator Structure") (NewCameraFOV :type "Float (single-precision)") (ReturnValue :type Boolean))
  (bind (_rotationadditive_roll _rotationadditive_pitch _rotationadditive_yaw) (`KismetMathLibrary.BreakRotator` (`self.RotationAdditive`)))
  (bind _asbp_character (cast `/Game/Rimanaru/Blueprints/CharacterAssets/BP_Character` CameraTarget))
  (bind _returnvalue (`SceneComponent.K2_GetComponentToWorld` (`/Game/Rimanaru/Blueprints/CharacterAssets/BP_Character.Camera` _asbp_character)))
  (return (+ (.location _returnvalue) (`self.LocationAdditive`)) (`KismetMathLibrary.MakeRotator` (+ _rotationadditive_roll (.roll (.rotation _returnvalue))) (+ (.pitch (.rotation _returnvalue)) _rotationadditive_pitch) (+ _rotationadditive_yaw (.yaw (.rotation _returnvalue)))) 90.0 true))

(fn `FResetTimeline`
  (params (TrackData :type "Float (double-precision)"))
  (if (and (== TrackData 0.0) (== (`self.isPlayerMoving`) false))
    (`self.ForceStop`)
    (else
      (set `self.Direction` (not (`self.Direction`)))
      (`self.StartHeadBobbing`))))

(fn `UserConstructionScript`)