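; BP_AnimNotifyItemSwap is an animation notify state that times the player character's item swap within an animation.
; On begin, it casts the mesh owner to BP_Character and calls SwapItemFunction.
; On end, it reaches BP_PlayerState through the character's stored reference and clears the item swapping status.
; Both events print debug strings.
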(fn `Received_NotifyBegin`
  (params (MeshComp :type "SkeletalMeshComponent Object Reference") (Animation :type "AnimSequenceBase Object Reference") (TotalDuration :type "Float (single-precision)") (EventReference :type "AnimNotifyEventReference Structure (by ref)"))
  (returns (ReturnValue :type Boolean))
  (bind _asbp_character (cast `/Game/Rimanaru/Blueprints/CharacterAssets/BP_Character` (`ActorComponent.GetOwner` MeshComp)))
  (`/Game/Rimanaru/Blueprints/CharacterAssets/BP_Character.SwapItemFunction` _asbp_character)
  (`KismetSystemLibrary.PrintString` null "BeginNotify")
  (return false))

(fn `Received_NotifyEnd`
  (params (MeshComp :type "SkeletalMeshComponent Object Reference") (Animation :type "AnimSequenceBase Object Reference") (EventReference :type "AnimNotifyEventReference Structure (by ref)"))
  (returns (ReturnValue :type Boolean))
  (bind _asbp_character (cast `/Game/Rimanaru/Blueprints/CharacterAssets/BP_Character` (`ActorComponent.GetOwner` MeshComp)))
  (bind _asbp_player_state (cast `/Game/Rimanaru/Blueprints/BP_PlayerState` (`/Game/Rimanaru/Blueprints/CharacterAssets/BP_Character.PlayerStateReference` _asbp_character)))
  (`/Engine/EditorBlueprintResources/StandardMacros.IsValid` _asbp_player_state
    (:`Is Valid`
      (`/Game/Rimanaru/Blueprints/BP_PlayerState.SetItemSwappingStatus` _asbp_player_state false)
      (`KismetSystemLibrary.PrintString` null "EndNotify")
      (return false))))