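; Player character Blueprint that handles basic mouse look and movement through Enhanced Input actions.
; Mouse input drives scaled yaw and pitch, with pitch inverted, while move input walks along control-rotation right and forward vectors, keeping forward movement level by ignoring pitch.
; A LerpInput helper scales input by elapsed time with a floor and upper cap, but the event graph does not call it.
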(event `EnhancedInput|/Game/Rimanaru/Inputs/MouseInput`
  (params (ActionValue :type "Vector2D Structure") (ElapsedSeconds :type "Float (double-precision)") (TriggeredSeconds :type "Float (double-precision)") (InputAction :type "InputAction Object Reference" :default "/Game/Rimanaru/Inputs/MouseInput.MouseInput"))
  (:`Triggered`
    (`self.AddControllerPitchInput` (* ActionValue_Y -0.5))
    (`self.AddControllerYawInput` (* ActionValue_X 0.5))))

(event `EnhancedInput|/Game/Rimanaru/Inputs/MoveButtons`
  (params (ActionValue :type "Vector2D Structure") (ElapsedSeconds :type "Float (double-precision)") (TriggeredSeconds :type "Float (double-precision)") (InputAction :type "InputAction Object Reference" :default "/Game/Rimanaru/Inputs/MoveButtons.MoveButtons"))
  (bind (_returnvalue_roll _returnvalue_pitch _returnvalue_yaw) (`KismetMathLibrary.BreakRotator` (`self.GetControlRotation`)))
  (bind (_returnvalue_roll_2 _returnvalue_pitch_2 _returnvalue_yaw_2) (`KismetMathLibrary.BreakRotator` (`self.GetControlRotation`)))
  (:`Triggered`
    (`self.AddMovementInput` (`KismetMathLibrary.GetRightVector` (`KismetMathLibrary.MakeRotator` _returnvalue_roll 0.0 _returnvalue_yaw)) ActionValue_X)
    (`self.AddMovementInput` (`KismetMathLibrary.GetForwardVector` (`KismetMathLibrary.MakeRotator` 0.0 0.0 _returnvalue_yaw_2)) ActionValue_Y)))

(fn `Lerp Input`
  (params (InputToLerp :type "Float (double-precision)") (TimeInput :type "Float (double-precision)"))
  (returns (LerpOutput :type "Float (double-precision)"))
  (locals (ChangeInput :type "Float (double-precision)") (MultiplierOfSpeed :type "Float (double-precision)" :default 3.0))
  (return (`KismetMathLibrary.FMin` 1.0 (* (`KismetMathLibrary.Lerp` 0.0 InputToLerp (`KismetMathLibrary.FMax` 0.4 (* TimeInput 1.8))) 0.8))))

(fn `UserConstructionScript`)